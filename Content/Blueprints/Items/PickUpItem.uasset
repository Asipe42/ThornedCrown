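; Pickup item actor that adds its item to the player's inventory on touch.
; When an actor tagged Player overlaps its capsule, it stores the character as owner, destroys itself and fires OnReceivedItem.
; That event passes the item to the owner's BP_PlayerController inventory and refreshes the HUD item slot.
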(event `self.Capsule.OnComponentBeginOverlap`
  (params (OverlappedComponent :type "PrimitiveComponent Object Reference") (OtherActor :type "Actor Object Reference") (OtherComp :type "PrimitiveComponent Object Reference") (OtherBodyIndex :type Integer) (bFromSweep :type Boolean) (SweepResult :type "HitResult Structure (by ref)"))
  (if (`self.ActorHasTag` OtherActor "Player")
    (bind _asbp_character (cast `/Game/Blueprints/BP_Character` OtherActor))
    (set `self.Onwer` _asbp_character)
    (`self.K2_DestroyActor`)
    (`self.On Received Item`)))

(event `On Received Item`
  (bind _asbp_player_controller (cast `/Game/Blueprints/BP_PlayerController` (`Pawn.GetController` (`self.Onwer`))))
  (`TCPlayerControllerBase.AddInventoryItem` _asbp_player_controller (`self.Item`) 1 1 true)
  (`/Game/Blueprints/Widgets/WB_HUD.Update Item Slot` (`/Game/Blueprints/BP_PlayerController.HUD` (`/Game/Blueprints/BP_BlueprintFunctionLibrary.GetPlayerControllerBP`))))

(fn `UserConstructionScript`)