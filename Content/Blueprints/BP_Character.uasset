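; Character Blueprint with melee combo helpers built on the Gameplay Ability System.
; IsUsingMelee reports whether any active ability carries the Ability.Melee tag.
; JumpMontageSection jumps the active montage to the section named by JumpSectionNotify when that notify is valid and IsPeriodCombo is set.
; DoMeleeAttack and the event graph are empty, and an unconnected next-section node remains unused.
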(fn `DoMeleeAttack`)

(fn `IsUsingMelee`
  (returns (Result :type Boolean))
  (return (> (`KismetArrayLibrary.Array_Length` (`self.GetActiveAbilitiesWithTags` (struct :`GameplayTags` (struct :`(TagName` "Ability.Melee"))))) 0)))

(fn `JumpMontageSection`
  (bind _returnvalue (`SkeletalMeshComponent.GetAnimInstance` (`self.Mesh`)))
  (`/Engine/EditorBlueprintResources/StandardMacros.IsValid` (`self.JumpSectionNotify`)
    (:`Is Valid`
      (if (`self.IsPeriodCombo`)
        (`AnimInstance.Montage_JumpToSection` _returnvalue (`/Game/Blueprints/AnimNotifies/AN_JumpSection.JumpSection` (`self.JumpSectionNotify`)) (`AnimInstance.GetCurrentActiveMontage` _returnvalue))))))

(fn `UserConstructionScript`)