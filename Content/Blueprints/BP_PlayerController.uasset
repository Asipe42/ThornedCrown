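; BP_PlayerController is the player's controller, handling Enhanced Input movement and look, plus HUD and weapon setup.
; BeginPlay adds the mapping context, creates the HUD and fills its weapon and potion slots, while Possess initializes the character's weapon.
; Move input is cached in MoveDirection, and Tick applies it as camera-relative movement.
; While a montage plays, Tick instead snaps the pawn's rotation to the camera-relative input direction.
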(event `self.ReceiveBeginPlay`
  ;[1 1 1] 초기화
  (`EnhancedInputSubsystemInterface.AddMappingContext` (subsystem `EnhancedInputLocalPlayerSubsystem`) "/Game/Input/IMC_Player.IMC_Player" 0 (struct))
  ;[1 1 1] HUD 초기화
  (if (`KismetSystemLibrary.IsValidClass` (`self.HUDClass`))
    (bind _returnvalue (`|CreateWidget` (`self.HUDClass`) self))
    (bind _output_get (set `self.HUD` _returnvalue))
    (`UserWidget.AddToViewport` _returnvalue 0)
    (`UserWidget.AddToViewport` _output_get 0)
    (`self.InitializeSlot` "/Game/Datas/Items/Weapons/Weapon_Axe.Weapon_Axe" "/Game/Datas/Items/Potions/Potion_Health.Potion_Health")
    (`/Game/Blueprints/Widgets/WB_HUD.Update Item Slot` (`self.HUD`))))

(event `self.ReceivePossess`
  (params (PossessedPawn :type "Pawn Object Reference"))
  ;[1 1 1] 무기 초기화
  (bind _asbp_player_character (cast `/Game/Blueprints/BP_PlayerCharacter` PossessedPawn))
  (bind _output_get (set `self.PlayerCharacter` _asbp_player_character))
  (`/Game/Blueprints/BP_PlayerCharacter.InitializeWeapon` _output_get))

(event `self.ReceiveTick`
  (params (DeltaSeconds :type "Float (single-precision)"))
  (bind _move_direction_x (`KismetMathLibrary.BreakVector2D` (`self.Move Direction`)))
  (bind (_move_direction_x_2 _move_direction_y) (`KismetMathLibrary.BreakVector2D` (`self.Move Direction`)))
  (bind (_move_direction_x_3 _move_direction_y_2) (`KismetMathLibrary.BreakVector2D` (`self.Move Direction`)))
  (bind _returnvalue (`KismetMathLibrary.MakeVector` _move_direction_y_2 _move_direction_x_3))
  (bind (_returnvalue_roll _returnvalue_pitch _returnvalue_yaw) (`KismetMathLibrary.BreakRotator` (`PlayerCameraManager.GetCameraRotation` (`GameplayStatics.GetPlayerCameraManager` 0))))
  (bind _returnvalue_2 (`PlayerCameraManager.GetCameraRotation` (`self.PlayerCameraManager`)))
  ;[1 1 1] 이동 및 회전
  (bind _ascharacter (cast `Character` (`self.K2_GetPawn`)))
  (if (`AnimInstance.Montage_IsPlaying` (`SkeletalMeshComponent.GetAnimInstance` (`Character.Mesh` _ascharacter)) null)
    ;;[1 1 1] 행동 중 회전
    (if (> (`KismetMathLibrary.VSize` _returnvalue) 0.0)
      (`self.K2_SetActorRotation` (`self.K2_GetPawn`) (`KismetMathLibrary.NormalizedDeltaRotator` (`KismetMathLibrary.MakeRotFromX` _returnvalue) (`KismetMathLibrary.MakeRotator` 0.0 0.0 (* _returnvalue_yaw -1.0))) false))
    (else
      ;;[1 1 1] 플레이어 캐릭터 이동
      (`Pawn.AddMovementInput` (`self.K2_GetPawn`) (`KismetMathLibrary.GetForwardVector` _returnvalue_2) _move_direction_y false)
      (`Pawn.AddMovementInput` (`self.K2_GetPawn`) (`KismetMathLibrary.GetRightVector` _returnvalue_2) _move_direction_x false))))

(event `EnhancedInput|/Game/Input/IA_Move`
  (params (ActionValue :type "Vector2D Structure") (ElapsedSeconds :type "Float (double-precision)") (TriggeredSeconds :type "Float (double-precision)") (InputAction :type "InputAction Object Reference" :default "/Game/Input/IA_Move.IA_Move"))
  ;[1 1 1] 이동 및 회전
  ;;[1 1 1] 플레이어 캐릭터 이동 감지
  (:`Triggered`
    (set `self.Move Direction` ActionValue :!label _label))
  (:`Completed`
    (goto _label)))

(event `EnhancedInput|/Game/Input/IA_Look`
  (params (ActionValue :type "Vector2D Structure") (ElapsedSeconds :type "Float (double-precision)") (TriggeredSeconds :type "Float (double-precision)") (InputAction :type "InputAction Object Reference" :default "/Game/Input/IA_Look.IA_Look"))
  ;[1 1 1] 이동 및 회전
  ;;[1 1 1] 카메라 회전
  (:`Triggered`
    (`self.AddYawInput` ActionValue_X)
    (`self.AddPitchInput` ActionValue_Y)))

(fn `UserConstructionScript`)